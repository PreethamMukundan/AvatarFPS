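; Earth character Blueprint that adds GAS-based hitbox damage and ability target confirmation.
; Its Box collision starts disabled after the parent BeginPlay, with a custom event to switch it to query-only.
; When the Box overlaps another AvatarCharacter, the server applies the ScarbDamageEffect gameplay effect to that character's ability system.
; The Z key confirms targeting on the character's own ability system.
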(event `self.ReceiveBeginPlay`
  (`parent.ReceiveBeginPlay`)
  (`self.DisableCollision`))

(event `Key|Z`
  (params (Key :type "Key Structure"))
  (:`Pressed`
    (`AbilitySystemComponent.TargetConfirm` (`self.AbilitySystemComp`))))

(event `self.Box.OnComponentBeginOverlap`
  (params (OverlappedComponent :type "PrimitiveComponent Object Reference") (OtherActor :type "Actor Object Reference") (OtherComp :type "PrimitiveComponent Object Reference") (OtherBodyIndex :type Integer) (bFromSweep :type Boolean) (SweepResult :type "HitResult Structure (by ref)"))
  (if (!= OtherActor self)
    (bind _asavatar_character (cast `AvatarCharacter` OtherActor))
    (`/Engine/EditorBlueprintResources/ActorMacros.Switch Has Authority`
      (:`Authority`
        (`KismetSystemLibrary.PrintString` "ApplyDamge")
        (`AbilitySystemComponent.BP_ApplyGameplayEffectToTarget` :`self` (`self.AbilitySystemComp`) :`GameplayEffectClass` "/Game/EARTH/ScarbDamageEffect.ScarbDamageEffect_C" :`Target` (`AvatarCharacter.AbilitySystemComp` _asavatar_character))))))

(event `DisableCollision`
  (`PrimitiveComponent.SetCollisionEnabled` (`self.Box`) "NoCollision"))

(event `xEnableCollision`
  (`PrimitiveComponent.SetCollisionEnabled` (`self.Box`) "QueryOnly"))

(fn `UserConstructionScript`)