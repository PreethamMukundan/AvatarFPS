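; BP_NatureCharacter is a character Blueprint that adds a NewWidgetBlueprint widget to the viewport on BeginPlay.
; An unconnected debug chain would line trace on the Camera channel along the FollowCamera's forward vector and draw a sphere at the impact point, but it never runs.
; Tick, overlap and construction logic are empty, and a Muzzle socket lookup is left unused.
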(event `self.ReceiveBeginPlay`
  (bind _returnvalue (`|CreateWidget` "/Game/NATURE/NewWidgetBlueprint.NewWidgetBlueprint_C"))
  (`UserWidget.AddToViewport` _returnvalue 0))

(event `self.ReceiveTick`
  (params (DeltaSeconds :type "Float (single-precision)")))

(fn `UserConstructionScript`)